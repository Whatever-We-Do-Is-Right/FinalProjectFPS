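; World map Blueprint that maps world locations into map space bounded by BottomLeft and UpRight corner actors.
; It derives map height from the corners' X distance and width from Y, and converts locations to absolute offsets from BottomLeft.
; A helper traces down on Visibility from a set height to find the surface point, falling back to the input.
; InitializeMap stores the player; click handling, map-to-world conversion and marker spawning are unimplemented or unconnected.
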(event Custom|InitializeMap
  (params (Player :type Actor%20Object%20Reference))
  (Utilities|IsValid Player
    (:Is%20Valid
      (Variables|Default|SetPlayer Player))))

(event Custom|OnMapClicked
  (params (Posistion :type Vector%202D%20Structure)))

(event EventBeginPlay)

(event EventTick
  (params (DeltaSeconds :type Float%20%28single-precision%29)))

(fn GetMapHeight
  (return (Math|Float|Absolute(Float) (- (.x (Transformation|GetActorLocation (Variables|Settings|GetUpRight))) (.x (Transformation|GetActorLocation (Variables|Settings|GetBottomLeft)))))))

(fn GetMapWidth
  (return (Math|Float|Absolute(Float) (- (.y (Transformation|GetActorLocation (Variables|Settings|GetUpRight))) (.y (Transformation|GetActorLocation (Variables|Settings|GetBottomLeft)))))))

(fn ConvertLocationtoMapLocation
  (params (Location :type Vector))
  (bind _bottomleft (Variables|Settings|GetBottomLeft))
  (bind _returnvalue (Transformation|GetActorLocation _bottomleft))
  (return (Math|Vector2D|MakeVector2D (Math|Float|Absolute(Float) (- (.x Location) (.x _returnvalue))) (Math|Float|Absolute(Float) (- (.y Location) (.y _returnvalue))))))

(fn TraceDownWorldLocation
  (params (In :type Vector))
  (LocalVariables|SetLocal_in In)
  (bind (_outhit _returnvalue) (Collision|LineTraceByChannel (Math|Vector|MakeVector (.x (LocalVariables|GetLocal_in)) (.y (LocalVariables|GetLocal_in)) (Variables|Settings|GetTraceDownHeight)) (LocalVariables|GetLocal_in) "TraceTypeQuery1" false 0 "None"))
  (if _returnvalue
    (return (.Location (Collision|BreakHitResult _outhit)))
    (else
      (return (LocalVariables|GetLocal_in)))))

(fn MapPositiontoWorldLocation)